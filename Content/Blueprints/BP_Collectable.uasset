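; Collectable actor that the player picks up with the Interact input while inside its Box trigger.
; Box overlaps with BP_PlayerBase enable and disable the actor's input.
; Interact decrements CollectablesLeft on BP_GameModeBase, shows a collectable widget, destroys the actor and plays a 2D pickup sound.
; On BeginPlay, each instance also creates a BP_HealthBar widget and adds it to the viewport.
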(event OnComponentBeginOverlap(Box)
  (params (OverlappedComponent :type Primitive%20Component%20Object%20Reference) (OtherActor :type Actor%20Object%20Reference) (OtherComp :type Primitive%20Component%20Object%20Reference) (OtherBodyIndex :type Integer) (bFromSweep :type Boolean) (SweepResult :type Hit%20Result%20Structure%20%28by%20ref%29))
  (Utilities|Casting|CastToBP_PlayerBase OtherActor)
  (Input|EnableInput (Game|GetPlayerController 0)))

(event OnComponentEndOverlap(Box)
  (params (OverlappedComponent :type Primitive%20Component%20Object%20Reference) (OtherActor :type Actor%20Object%20Reference) (OtherComp :type Primitive%20Component%20Object%20Reference) (OtherBodyIndex :type Integer))
  (Utilities|Casting|CastToBP_PlayerBase OtherActor)
  (Input|DisableInput (Game|GetPlayerController 0)))

(event Custom|CreateUI
  ;[1 1 1] HealthBar
  (bind _returnvalue (UserInterface|CreateWidget "/Game/UI/BP_HealthBar.BP_HealthBar_C" (Game|GetPlayerController 0)))
  (bind _output_get (Variables|Default|SetHelathBar _returnvalue))
  (UserInterface|Viewport|AddtoViewport _output_get 0))

(event EventBeginPlay
  (CallFunction|CreateUI))

(event Input|ActionEvents|InputActionInteract
  (params (Key :type Key%20Structure :default "None"))
  (:Pressed
    (Utilities|FlowControl|Sequence
      (:then_0
        (bind _asbp_game_mode_base (Utilities|Casting|CastToBP_GameModeBase (Game|GetGameMode)))
        (bind _result (Math|Integer|DecrementInt (Variables|/Game/Blueprints/BP_GameModeBase.BP_GameModeBase_C|GetCollectablesLeft _asbp_game_mode_base))
          (:%20%20
            (bind _output_get (Variables|/Game/Blueprints/BP_GameModeBase.BP_GameModeBase_C|SetCollectablesLeft _asbp_game_mode_base _result))
            (bind _returnvalue (UserInterface|CreateWidget "/Game/UI/BP_CollectableWidget.BP_CollectableWidget_C"))
            (UserInterface|Viewport|AddtoViewport _returnvalue 0)
            (Actor|DestroyActor))))
      (:then_1
        (Audio|PlaySound2D "/Game/Audio/PickingUpCloudCue.PickingUpCloudCue" 3.5 1.0 0.0 0 0)))))

(fn ConstructionScript)