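; BP_DoorOpen is a door that the player opens with E once no collectables are left.
; A box trigger enables the door's input while a BP_PlayerBase overlaps it and disables it on exit.
; Pressing E checks the remaining count on BP_GameModeBase, then plays a timeline that rotates the door mesh's yaw and sets a GameOver flag on each update.
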(event OnComponentBeginOverlap(Box)
  (params (OverlappedComponent :type Primitive%20Component%20Object%20Reference) (OtherActor :type Actor%20Object%20Reference) (OtherComp :type Primitive%20Component%20Object%20Reference) (OtherBodyIndex :type Integer) (bFromSweep :type Boolean) (SweepResult :type Hit%20Result%20Structure%20%28by%20ref%29))
  (Utilities|Casting|CastToBP_PlayerBase OtherActor)
  (Input|EnableInput (Game|GetPlayerController 0)))

(event OnComponentEndOverlap(Box)
  (params (OverlappedComponent :type Primitive%20Component%20Object%20Reference) (OtherActor :type Actor%20Object%20Reference) (OtherComp :type Primitive%20Component%20Object%20Reference) (OtherBodyIndex :type Integer))
  (Utilities|Casting|CastToBP_PlayerBase OtherActor)
  (Input|DisableInput (Game|GetPlayerController 0)))

(event Input|KeyboardEvents|E
  (params (Key :type Key%20Structure :default "None"))
  (:Pressed
    (bind _asbp_game_mode_base (Utilities|Casting|CastToBP_GameModeBase (Game|GetGameMode)))
    (if (== (Variables|/Game/Blueprints/BP_GameModeBase.BP_GameModeBase_C|GetCollectablesLeft _asbp_game_mode_base) 0)
      (bind _doorturn (Timeline|DoorOpen Play)
        (:Update
          (Transformation|SetRelativeRotation (Variables|Default|GetSM_Door) (Math|Rotator|MakeRotator 0.0 0.0 _doorturn) false false)
          (Variables|Default|SetGameOver true))))))

(fn ConstructionScript)